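; BP_troopMover issues move or attack orders to a group of troops based on where the camera points.
; Its giveCommand event stores the troops and traces WorldDynamic objects forward from the camera.
; A hit on BP_HexGrid sends each Troop1 to the impact point, while a hit on BP_attackThis sets each to attack that actor.
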(event Custom|giveCommand
  (params (troops :type Array%20of%20Actor%20Object%20References) (camera :type BP%20Camera%20Pawn%203%20Object%20Reference))
  (bind _camera (Variables|/Game/Camera3/BP_CameraPawn3.BP_CameraPawn3_C|GetCamera camera))
  (bind _returnvalue (Transformation|GetWorldLocation _camera))
  (Variables|Default|SetTroops troops)
  (bind _outhit (Collision|LineTraceForObjects _returnvalue (+ _returnvalue (* (Math|Vector|GetForwardVector _camera) 2.5e+03)) (Utilities|Array|MakeArray "ObjectTypeQuery2") false 0 "None"))
  (Utilities|Casting|CastToBP_HexGrid (.HitActor (Collision|BreakHitResult _outhit))
    (:then
      (for _array_element (Variables|Default|GetTroops)
        (bind _astroop_1 (Utilities|Casting|CastToTroop1 _array_element))
        (Default|SetStateMovetoLocation _astroop_1 (.ImpactPoint (Collision|BreakHitResult _outhit)))))
    (:CastFailed
      (bind _asbp_attack_this (Utilities|Casting|CastToBP_attackThis (.HitActor (Collision|BreakHitResult _outhit))))
      (for _array_element_2 (Variables|Default|GetTroops)
        (bind _astroop_1_2 (Utilities|Casting|CastToTroop1 _array_element_2))
        (Default|SetStateAttack _astroop_1_2 _asbp_attack_this)))))

(fn ConstructionScript)